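; BP_PlayerCharacter is the player character, handling movement, look, shooting, aiming and weapon interaction through Enhanced Input.
; Aiming plays a timeline that lerps the camera from its initial position toward the offset WeaponSlot location, reversing on release.
; Capsule overlaps set the current Interactable, cleared on any end overlap.
; Interact possesses a BP_StaticWeapon, or attaches a BP_Weapon to WeaponSlot after destroying any held weapon.
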(event OnComponentBeginOverlap(CapsuleComponent)
  (params (OverlappedComponent :type Primitive%20Component%20Object%20Reference) (OtherActor :type Actor%20Object%20Reference) (OtherComp :type Primitive%20Component%20Object%20Reference) (OtherBodyIndex :type Integer) (bFromSweep :type Boolean) (SweepResult :type Hit%20Result%20Structure%20%28by%20ref%29))
  (Variables|Default|SetInteractable OtherActor))

(event Input|EnhancedActionEvents|EnhancedInputActionIA_Movement
  (params (ActionValue :type Vector%202D%20Structure) (ElapsedSeconds :type Float%20%28double-precision%29) (TriggeredSeconds :type Float%20%28double-precision%29) (InputAction :type Input%20Action%20Object%20Reference :default "/Game/Characters/Inputs/IA_Movement.IA_Movement"))
  (Pawn|Input|AddMovementInput (Transformation|GetActorForwardVector) (.x ActionValue) false)
  (Pawn|Input|AddMovementInput (Transformation|GetActorRightVector) (.y ActionValue) false))

(event Input|EnhancedActionEvents|EnhancedInputActionIA_Look
  (params (ActionValue :type Vector%202D%20Structure) (ElapsedSeconds :type Float%20%28double-precision%29) (TriggeredSeconds :type Float%20%28double-precision%29) (InputAction :type Input%20Action%20Object%20Reference :default "/Game/Characters/Inputs/IA_Look.IA_Look"))
  (Pawn|Input|AddControllerYawInput (.x ActionValue))
  (Pawn|Input|AddControllerPitchInput (.y ActionValue)))

(event Input|EnhancedActionEvents|EnhancedInputActionIA_Shoot
  (params (ActionValue :type Boolean) (ElapsedSeconds :type Float%20%28double-precision%29) (TriggeredSeconds :type Float%20%28double-precision%29) (InputAction :type Input%20Action%20Object%20Reference :default "/Game/Characters/Inputs/IA_Shoot.IA_Shoot"))
  (bind _handweapon (Variables|Default|GetHandWeapon))
  (:Triggered
    (Utilities|IsValid _handweapon
      (:Is%20Valid
        (Default|Shoot _handweapon))))
  (:Completed
    (Utilities|IsValid _handweapon
      (:Is%20Valid
        (Default|Stop _handweapon)))))

(event Input|EnhancedActionEvents|EnhancedInputActionIA_Interact
  (params (ActionValue :type Boolean) (ElapsedSeconds :type Float%20%28double-precision%29) (TriggeredSeconds :type Float%20%28double-precision%29) (InputAction :type Input%20Action%20Object%20Reference :default "/Game/Characters/Inputs/IA_Interact.IA_Interact"))
  (bind _asbp_static_weapon (Utilities|Casting|CastToBP_StaticWeapon (Variables|Default|GetInteractable))
    (:then
      (Pawn|Possess (Game|GetPlayerController 0) _asbp_static_weapon))
    (:CastFailed
      (bind _asbp_hand_weapon (Utilities|Casting|CastToBP_Weapon (Variables|Default|GetInteractable)))
      (Utilities|IsValid (Variables|Default|GetHandWeapon)
        (:Is%20Valid
          (Actor|DestroyActor (Variables|Default|GetHandWeapon)))
        (:Is%20Not%20Valid
          _))
      (Utilities|IsValid _asbp_hand_weapon
        (:Is%20Valid
          (bind _output_get (Variables|Default|SetHandWeapon _asbp_hand_weapon))
          (Transformation|AttachComponentToComponent _output_get (Variables|Default|GetWeaponSlot) "None" "SnapToTarget" "SnapToTarget" "KeepRelative" true))))))

(event Input|EnhancedActionEvents|EnhancedInputActionIA_Aim
  (params (ActionValue :type Boolean) (ElapsedSeconds :type Float%20%28double-precision%29) (TriggeredSeconds :type Float%20%28double-precision%29) (InputAction :type Input%20Action%20Object%20Reference :default "/Game/Characters/Inputs/IA_Aim.IA_Aim"))
  (:Started
    (bind _aimtime (Timeline|Timeline Play)
      (:Update
        (Transformation|SetRelativeLocation (Variables|Default|GetCamera) (Math|Vector|Lerp(Vector) (Variables|Default|GetInitalCameraLocation) (+ (Variables|Default|GetAimOffset) (Variables|/Script/Engine.SceneComponent|GetRelativeLocation (Variables|Default|GetWeaponSlot))) _aimtime) true false))))
  (:Canceled
    (Timeline|Timeline Reverse))
  (:Completed
    (Timeline|Timeline Reverse)))

(event EventBeginPlay
  (Variables|Default|SetInitalCameraLocation (Variables|/Script/Engine.SceneComponent|GetRelativeLocation (Variables|Default|GetCamera))))

(event Collision|EventActorEndOverlap
  (params (OtherActor :type Actor%20Object%20Reference))
  (Variables|Default|SetInteractable 0))

(fn ConstructionScript)