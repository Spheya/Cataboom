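; BP_FlameThrower is a weapon Blueprint that fires a flame and blows up enemies caught in its reach.
; Shoot activates the Flame component once through a DoOnce, then on every call runs a debug-drawn capsule trace from the Muzzle along the actor's forward vector out to Range.
; Each BP_EnemyAI hit receives ExplodeKitten, with no projectile spawned in this logic.
; Stop deactivates the flame and resets the DoOnce.
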(event EventBeginPlay
  (|CallParentFunction) ; This node is disabled and will not be called.\nDrag off pins to build functionality.
)

(event Collision|EventActorBeginOverlap
  (params (OtherActor :type Actor%20Object%20Reference))
  (|CallParentFunction OtherActor) ; This node is disabled and will not be called.\nDrag off pins to build functionality.
)

(event EventTick
  (params (DeltaSeconds :type Float%20%28single-precision%29))
  (|CallParentFunction DeltaSeconds) ; This node is disabled and will not be called.\nDrag off pins to build functionality.
)

(event EventStop
  (bind _flame (Variables|Default|GetFlame))
  (Components|Activation|SetActive _flame false false)
  (Utilities|FlowControl|DoOnce false) ; enters at Reset
)

(event EventShoot
  (bind _muzzle (Variables|Default|GetMuzzle))
  (bind _returnvalue (Transformation|GetWorldLocation _muzzle))
  (Utilities|FlowControl|Sequence
    (:then_0
      (Utilities|FlowControl|DoOnce false
        (:Completed
          (Components|Activation|SetActive (Variables|Default|GetFlame) true false))))
    (:then_1
      (bind _outhits (Class|KismetSystemLibrary|CapsuleTraceMulti _returnvalue (+ _returnvalue (* (Transformation|GetActorForwardVector) (Variables|Default|GetRange))) 1.5e+02 3e+01 "TraceTypeQuery1" false 0 "ForOneFrame" true))
      (for _array_element _outhits
        (bind _asbp_enemy_ai (Utilities|Casting|CastToBP_EnemyAI (.HitActor (Collision|BreakHitResult _array_element))))
        (Default|ExplodeKitten _asbp_enemy_ai)))))

(fn ConstructionScript
  (|CallParentFunction))

(fn SpawnMuzzle
  (|CallParentFunction))

(fn SpawnProjectile
  (|CallParentFunction))