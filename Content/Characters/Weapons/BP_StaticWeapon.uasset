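; BP_StaticWeapon is a possessable mounted weapon that the player aims and fires.
; On BeginPlay it spawns the configured WeaponClass and snaps it onto the WeaponSlot component.
; Enhanced Input drives controller yaw and pitch for look, and forwards shoot input to the spawned weapon's Shoot and Stop.
; Interact hands possession back to the BP_PlayerCharacter found in the world.
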(event Input|EnhancedActionEvents|EnhancedInputActionIA_Interact
  (params (ActionValue :type Boolean) (ElapsedSeconds :type Float%20%28double-precision%29) (TriggeredSeconds :type Float%20%28double-precision%29) (InputAction :type Input%20Action%20Object%20Reference :default "/Game/Characters/Inputs/IA_Interact.IA_Interact"))
  (bind _returnvalue (Actor|GetActorOfClass "/Game/Characters/BP_PlayerCharacter.BP_PlayerCharacter_C"))
  (Pawn|Possess (Pawn|GetController) _returnvalue))

(event Input|EnhancedActionEvents|EnhancedInputActionIA_Look
  (params (ActionValue :type Vector%202D%20Structure) (ElapsedSeconds :type Float%20%28double-precision%29) (TriggeredSeconds :type Float%20%28double-precision%29) (InputAction :type Input%20Action%20Object%20Reference :default "/Game/Characters/Inputs/IA_Look.IA_Look"))
  (Pawn|Input|AddControllerYawInput (.x ActionValue))
  (Pawn|Input|AddControllerPitchInput (.y ActionValue)))

(event Input|EnhancedActionEvents|EnhancedInputActionIA_Shoot
  (params (ActionValue :type Boolean) (ElapsedSeconds :type Float%20%28double-precision%29) (TriggeredSeconds :type Float%20%28double-precision%29) (InputAction :type Input%20Action%20Object%20Reference :default "/Game/Characters/Inputs/IA_Shoot.IA_Shoot"))
  (bind _weapon (Variables|Default|GetWeapon))
  (:Triggered
    (Default|Shoot _weapon))
  (:Completed
    (Default|Stop _weapon)))

(event EventBeginPlay
  (bind _returnvalue (Game|SpawnActorfromClass (Variables|Default|GetWeaponClass) (Transformation|GetWorldTransform (Variables|Default|GetDefaultSceneRoot)) "Undefined" "MultiplyWithRoot" 0 0))
  (bind _output_get (Variables|Default|SetWeapon _returnvalue))
  (Transformation|AttachComponentToComponent _output_get (Variables|Default|GetWeaponSlot) "None" "SnapToTarget" "SnapToTarget" "KeepRelative" true))

(fn ConstructionScript)