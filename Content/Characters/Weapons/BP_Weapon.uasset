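; Weapon actor that fires projectiles along the player camera's rotation and plays a Niagara muzzle effect.
; Shoot spawns a projectile at the muzzle plus a camera-rotated GunOffset, with a DoOnce reset by a FireRate timer limiting the rate.
; A second DoOnce activates the muzzle effect on the first shot only, until Stop deactivates it and re-arms it.
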(event Custom|Shoot
  (Utilities|FlowControl|DoOnce false
    (:Completed
      (CallFunction|SpawnProjectile)
      (Utilities|Time|SetTimerbyEvent (delegate Custom|Cooldown) (Variables|Default|GetFireRate))
      (Utilities|FlowControl|DoOnce false
        (:Completed
          (CallFunction|SpawnMuzzle))))))

(event Custom|Stop
  (Components|Activation|SetActive (Variables|Default|GetMuzzle) false false)
  (Utilities|FlowControl|DoOnce false) ; enters at Reset
)

(event Custom|Cooldown
  (Utilities|FlowControl|DoOnce false) ; enters at Reset
)

(event EventBeginPlay)

(event Collision|EventActorBeginOverlap
  (params (OtherActor :type Actor%20Object%20Reference)))

(event EventTick
  (params (DeltaSeconds :type Float%20%28single-precision%29)))

(fn ConstructionScript)

(fn SpawnProjectile
  (bind _returnvalue (Game|GetPlayerCameraManager 0))
  (bind _returnvalue_2 (Camera|GetCameraRotation _returnvalue))
  (Game|SpawnActorfromClass (Variables|Default|GetProjectile) (Math|Transform|MakeTransform (+ (Transformation|GetWorldLocation (Variables|Default|GetMuzzle)) (Math|Vector|RotateVector (Variables|Default|GetGun%20Offset) _returnvalue_2)) _returnvalue_2 "1.000000,1.000000,1.000000") "AdjustIfPossibleButDontSpawnIfColliding" "SelectDefaultAtRuntime" 0 0))

(fn SpawnMuzzle
  (bind _muzzle (Variables|Default|GetMuzzle))
  (Class|NiagaraComponent|SetAsset _muzzle (Variables|Default|GetMuzzleFX) true)
  (Components|Activation|SetActive _muzzle true false))