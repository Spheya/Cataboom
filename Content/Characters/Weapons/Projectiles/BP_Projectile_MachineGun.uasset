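; Machine gun projectile actor that works as a hitscan shot rather than a moving projectile.
; On BeginPlay it line-traces forward over Range on the Visibility channel, with a brief debug line drawn.
; Only a BP_EnemyAI hit triggers ExplodeKitten, activates Hiteffects at the impact point, spawns ImpactActor there and destroys the projectile.
; Misses and other hits leave the actor alive in this graph.
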(event EventBeginPlay
  (bind _returnvalue (Transformation|GetActorLocation))
  (bind _hiteffects (Variables|Default|GetHiteffects))
  (bind (_outhit _returnvalue_2) (Collision|LineTraceByChannel _returnvalue (+ _returnvalue (* (Transformation|GetActorForwardVector) (Variables|Default|GetRange))) "TraceTypeQuery1" false 0 "ForDuration" true "(R=1.000000,G=0.000000,B=0.000000,A=1.000000)" "(R=0.000000,G=1.000000,B=0.000000,A=1.000000)" 0.1))
  (if _returnvalue_2
    (bind _asbp_enemy_ai (Utilities|Casting|CastToBP_EnemyAI (.HitActor (Collision|BreakHitResult _outhit))))
    (Default|ExplodeKitten _asbp_enemy_ai)
    (Components|Activation|SetActive _hiteffects true false)
    (Transformation|SetWorldLocation _hiteffects (.ImpactPoint (Collision|BreakHitResult _outhit)) false false)
    (Game|SpawnActorfromClass (Variables|Default|GetImpactActor) (Math|Transform|MakeTransform (.ImpactPoint (Collision|BreakHitResult _outhit))) "AlwaysSpawn" "SelectDefaultAtRuntime" 0 0)
    (Actor|DestroyActor)))

(fn ConstructionScript)