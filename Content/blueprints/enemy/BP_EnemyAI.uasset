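; Enemy cat character, drawn as a camera-facing billboard, with a randomized look and adjustable walk speed.
; Construction gives CatGraphics a dynamic material with a random CatID and color seed for per-instance variation.
; Tick turns CatGraphics toward the player camera on the horizontal plane by flattening Z and offsetting yaw.
; ExplodeKitten simply destroys the actor, and UpdateWalkSpeed sets the movement component's max walk speed.
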(event Custom|ExplodeKitten
  (Actor|DestroyActor))

(event EventTick
  (params (DeltaSeconds :type Float%20%28single-precision%29))
  (bind _returnvalue (Game|GetPlayerCameraManager 0))
  (bind _catgraphics (Variables|Default|GetCatGraphics))
  (bind _returnvalue_2 (Camera|GetCameraLocation _returnvalue))
  (bind _returnvalue_3 (Transformation|GetWorldLocation _catgraphics))
  (bind _returnvalue_4 (* _returnvalue_2 "1.000000,1.000000,0.000000"))
  (bind _returnvalue_5 (* _returnvalue_3 "1.000000,1.000000,0.000000"))
  (bind _returnvalue_6 (Math|Rotator|FindLookatRotation _returnvalue_4 _returnvalue_5))
  (bind (_roll _pitch _yaw) (Math|Rotator|BreakRotator _returnvalue_6))
  (Transformation|SetWorldRotation (Variables|Default|GetCatGraphics) (Math|Rotator|MakeRotator _roll _pitch (+ _yaw 9e+01)) false false))

(fn ConstructionScript
  (bind _returnvalue (Rendering|Material|CreateDynamicMaterialInstance "/Game/Materials/CatMaterial.CatMaterial" "None" "None" :!class /Script/Engine.KismetMaterialLibrary))
  (Rendering|Material|SetScalarParameterValue _returnvalue "CatID" (Math|Conversions|ToFloat(Integer) (Math|Random|RandomInteger 4)) :!class /Script/Engine.MaterialInstanceDynamic)
  (Rendering|Material|SetVectorParameterValue _returnvalue "Seed" (Math|Color|MakeColor (Math|Random|RandomFloat) (Math|Random|RandomFloat) (Math|Random|RandomFloat) (Math|Random|RandomFloat)) :!class /Script/Engine.MaterialInstanceDynamic)
  (Rendering|Material|SetMaterial (Variables|Default|GetCatGraphics) 0 _returnvalue))

(fn UpdateWalkSpeed
  (params (NewWalkSpeed :type Float%20%28double-precision%29))
  (Variables|/Script/Engine.CharacterMovementComponent|SetMaxWalkSpeed (Variables|Character|GetCharacterMovement) NewWalkSpeed))